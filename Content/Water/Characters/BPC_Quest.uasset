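; BPC_Quest is a quest component that shows the active quest's name on screen.
; On BeginPlay it creates a WBP_OnQuest widget, adds it to the viewport and keeps a reference to it.
; Two events drive the widget's text: one writes the ActiveQuest name, the other clears it.
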(event Custom|SetActiveQuestText
  (Rendering|Components|TextRender|SetText (Variables|/Game/Water/UI/WBP_OnQuest.WBP_OnQuest_C|GetActiveQuestText (Variables|Default|GetOnQuestWidget)) (Utilities|Text|ToText(String) (.Name (Utilities|Struct|BreakS_Quest (Variables|Default|GetActiveQuest))))))

(event Custom|SetBlankQuestText
  (Rendering|Components|TextRender|SetText (Variables|/Game/Water/UI/WBP_OnQuest.WBP_OnQuest_C|GetActiveQuestText (Variables|Default|GetOnQuestWidget)) ""))

(event EventBeginPlay
  (bind _returnvalue (UserInterface|CreateWidget "/Game/Water/UI/WBP_OnQuest.WBP_OnQuest_C"))
  (bind _output_get (Variables|Default|SetOnQuestWidget _returnvalue))
  (UserInterface|Viewport|AddtoViewport _output_get 0))