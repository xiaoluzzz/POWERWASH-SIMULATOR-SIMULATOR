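; BP_Gun is a gun pickup that grants the WaterGirlCharacter its first gun.
; Player overlap with its Sphere shows a Widget, enables input on the actor and opens a Gate; leaving only hides the Widget.
; IA_Interact passes through that Gate, casts the overlapped actor to WaterGirlCharacter, sets PlayerHasGun1 and destroys the pickup.
; The Gate and input stay enabled after overlap ends.
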(event OnComponentBeginOverlap(Sphere)
  (params (OverlappedComponent :type Primitive%20Component%20Object%20Reference) (OtherActor :type Actor%20Object%20Reference) (OtherComp :type Primitive%20Component%20Object%20Reference) (OtherBodyIndex :type Integer) (bFromSweep :type Boolean) (SweepResult :type Hit%20Result%20Structure%20%28by%20ref%29))
  (if (== OtherActor (Game|Player|GetPlayerPawn 0))
    (Rendering|SetVisibility (Variables|Default|GetWidget) true false)
    (Input|EnableInput (Game|GetPlayerController 0))
    (Utilities|FlowControl|Gate true) ; enters at Open
  ))

(event OnComponentEndOverlap(Sphere)
  (params (OverlappedComponent :type Primitive%20Component%20Object%20Reference) (OtherActor :type Actor%20Object%20Reference) (OtherComp :type Primitive%20Component%20Object%20Reference) (OtherBodyIndex :type Integer))
  (Rendering|SetVisibility (Variables|Default|GetWidget) false false))

(event Input|EnhancedActionEvents|EnhancedInputActionIA_Interact
  (params (ActionValue :type Boolean) (ElapsedSeconds :type Float%20%28double-precision%29) (TriggeredSeconds :type Float%20%28double-precision%29) (InputAction :type Input%20Action%20Object%20Reference :default "/Game/ThirdPerson/Input/Actions/IA_Interact.IA_Interact"))
  (:Started
    (Utilities|FlowControl|Gate true
      (:Exit
        (bind _aswater_girl_character (Utilities|Casting|CastToWaterGirlCharacter (stale OnComponentBeginOverlap(Sphere) OtherActor)))
        (Variables|/Game/Water/Characters/WaterGirlCharacter.WaterGirlCharacter_C|SetPlayerHasGun1 _aswater_girl_character true)
        (Actor|DestroyActor)))))

(event EventBeginPlay)

(event Collision|EventActorBeginOverlap
  (params (OtherActor :type Actor%20Object%20Reference)))

(event EventTick
  (params (DeltaSeconds :type Float%20%28single-precision%29)))

(fn ConstructionScript)