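; BP_Desk is an interactable desk that presents its list of quests to the player.
; A box overlap by the player pawn shows a widget component and enables input on the actor; leaving only hides the widget.
; Interact toggles a WBP_Desk screen, filling it from the Quests array and switching cursor and input mode.
; The screen receives a reference to the desk, and CloseQuestWidget reuses the closing branch.
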(event OnComponentBeginOverlap(Box)
  (params (OverlappedComponent :type Primitive%20Component%20Object%20Reference) (OtherActor :type Actor%20Object%20Reference) (OtherComp :type Primitive%20Component%20Object%20Reference) (OtherBodyIndex :type Integer) (bFromSweep :type Boolean) (SweepResult :type Hit%20Result%20Structure%20%28by%20ref%29))
  (if (== OtherActor (Game|Player|GetPlayerPawn 0))
    (Rendering|SetVisibility (Variables|Default|GetWidget) true false)
    (Input|EnableInput (Game|GetPlayerController 0))))

(event OnComponentEndOverlap(Box)
  (params (OverlappedComponent :type Primitive%20Component%20Object%20Reference) (OtherActor :type Actor%20Object%20Reference) (OtherComp :type Primitive%20Component%20Object%20Reference) (OtherBodyIndex :type Integer))
  (Rendering|SetVisibility (Variables|Default|GetWidget) false false))

(event Custom|CloseQuestWidget
  (bind _returnvalue (Game|GetPlayerController 0))
  (Widget|RemovefromParent (Variables|Default|GetQuestWidget))
  (Variables|Default|SetQuestWidget 0)
  (Variables|/Script/Engine.PlayerController|SetbShowMouseCursor _returnvalue false)
  (Input|SetInputModeGameOnly _returnvalue false)
  (Variables|Default|SetQuestWidgetActive false))

(event EventBeginPlay)

(event Collision|EventActorBeginOverlap
  (params (OtherActor :type Actor%20Object%20Reference)))

(event EventTick
  (params (DeltaSeconds :type Float%20%28single-precision%29)))

(event EventInteract
  (bind _returnvalue (Game|GetPlayerController 0))
  (bind _returnvalue_2 (Game|GetPlayerController 0))
  (if (not (Variables|Default|GetQuestWidgetActive))
    (bind _returnvalue_3 (UserInterface|CreateWidget "/Game/Water/UI/WBP_Desk.WBP_Desk_C"))
    (bind _output_get (Variables|Default|SetQuestWidget _returnvalue_3))
    (UserInterface|Viewport|AddtoViewport _output_get 0)
    (Variables|Default|SetQuestWidgetActive true)
    (Variables|/Script/Engine.PlayerController|SetbShowMouseCursor _returnvalue true)
    (Input|SetInputModeGameandUI _returnvalue (Variables|Default|GetQuestWidget) "DoNotLock" true false)
    (Variables|/Game/Water/UI/WBP_Desk.WBP_Desk_C|SetDeskBP (Variables|Default|GetQuestWidget) self)
    (for _array_element (Variables|Default|GetQuests)
      (Default|AddQuest (Variables|Default|GetQuestWidget) _array_element))
    (else
      (Widget|RemovefromParent (Variables|Default|GetQuestWidget))
      (Variables|Default|SetQuestWidget 0)
      (Variables|/Script/Engine.PlayerController|SetbShowMouseCursor _returnvalue_2 false)
      (Input|SetInputModeGameOnly _returnvalue_2 false)
      (Variables|Default|SetQuestWidgetActive false))))

(fn ConstructionScript)