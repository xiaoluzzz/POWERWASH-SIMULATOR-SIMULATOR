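; Enemy actor that sets up render-target-based hit masking on its skeletal mesh.
; On BeginPlay it creates dynamic instances of the enemy and hit materials, plus two render targets.
; A scene capture limited to this actor writes the unwrap target, which feeds the hit material.
; The cleared hit target feeds the mesh material; nothing here paints hits into it.
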(event EventBeginPlay
  (bind _returnvalue (Rendering|Material|CreateDynamicMaterialInstance (Variables|Default|GetSkeletalMesh) 0 "/Game/Water/Materials/M_enemy.M_enemy" "None" :!class /Script/Engine.PrimitiveComponent))
  (Variables|Default|SetMID_Original _returnvalue)
  (bind _returnvalue_2 (Rendering|Material|CreateDynamicMaterialInstance "/Game/Water/Materials/M_Hit.M_Hit" "None" "None" :!class /Script/Engine.KismetMaterialLibrary))
  (Variables|Default|SetMID_Hit _returnvalue_2)
  (Utilities|FlowControl|Sequence
    (:then_0
      (bind _returnvalue_3 (Rendering|CreateRenderTarget2D 1024 1024 "RTF_RGBA16f"))
      (bind _output_get (Variables|Default|SetRT_Unwrap _returnvalue_3))
      (Variables|/Script/Engine.SceneCaptureComponent2D|SetTextureTarget (Variables|Default|GetSceneCaptureComponent2D) _output_get)
      (Rendering|Material|SetTextureParameterValue (Variables|Default|GetMID_Hit) "Unwrap" (Variables|Default|GetRT_Unwrap))
      (Rendering|SceneCapture|ShowOnlyActorComponents (Variables|Default|GetScene%20Capture%20Component%202D) self false))
    (:then_1
      (bind _returnvalue_4 (Rendering|CreateRenderTarget2D 1024 1024 "RTF_RGBA16f"))
      (Variables|Default|SetRT_Hit _returnvalue_4)
      (Rendering|Material|SetTextureParameterValue (Variables|Default|GetMID_Original) "Hit" (Variables|Default|GetRT_Hit))
      (Rendering|ClearRenderTarget2D (Variables|Default|GetRT_Hit)))))

(event Collision|EventActorBeginOverlap
  (params (OtherActor :type Actor%20Object%20Reference)))

(fn ConstructionScript)