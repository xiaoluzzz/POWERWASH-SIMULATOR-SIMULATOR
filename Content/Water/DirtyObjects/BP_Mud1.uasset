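; BP_Mud1 is a cleanable mud decal that rewards the WaterGirlCharacter with money and a mud count when fully cleaned.
; Each Ray call triggers get, which plays a timeline that drives the OP parameter on the decal's dynamic material.
; A short Delay on Update stops the timeline, so cleaning advances in increments under repeated calls.
; On completion it destroys the Box component and grants the rewards.
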(event Custom|get
  (bind _新建轨道_0 (Timeline|时间轴 Play)
    (:Update
      (Utilities|FlowControl|Delay 0.1)
      (Utilities|FlowControl|Sequence
        (:then_0
          (Timeline|时间轴 Stop))
        (:then_1
          (Rendering|Material|SetScalarParameterValue (Variables|Default|GetO) "OP" _新建轨道_0 :!class /Script/Engine.MaterialInstanceDynamic))))
    (:Finished
      (Components|DestroyComponent (Variables|Default|GetBox))
      (Utilities|FlowControl|Sequence
        (:then_0
          (bind _returnvalue (Actor|GetActorOfClass "/Game/Water/Characters/WaterGirlCharacter.WaterGirlCharacter_C"))
          (Default|AddMoney _returnvalue 5))
        (:then_1
          (bind _returnvalue_2 (Actor|GetActorOfClass "/Game/Water/Characters/WaterGirlCharacter.WaterGirlCharacter_C"))
          (Default|AddMudCount _returnvalue_2 1))))))

(event EventBeginPlay
  (bind _returnvalue (Rendering|Material|CreateDynamicMaterialInstance (Variables|Default|GetDecal) :!class /Script/Engine.DecalComponent))
  (Variables|Default|SetO _returnvalue))

(fn ConstructionScript)

(fn Ray
  (CallFunction|Get))